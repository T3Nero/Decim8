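; Blueprint function library for the Nice Settings Menu, giving global access to the player controller's settings component.
; Navigation wrappers fetch that component and, if valid, forward input, actions, apply, restore, reset, info and section switching.
; Helpers play a cooldown-gated click sound and find a text's array index.
; Another sets resolution and window mode via r.SetRes, optionally clamped to desktop size, skipping repeats and re-executing after a delay.
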(fn GetNSMPCComponent
  ;[1 1 1] Return reference to Nice Settings Menu PC component from player controller
  (return (Actor|GetComponentbyClass (Game|GetPlayerController 0) "/Game/NiceSettingsMenu/Blueprints/AC_PC_NiceSettingsComponent.AC_PC_NiceSettingsComponent_C")))

(fn NiceNaviagtionInput
  (params (Direction :type E_NiceNavigationDirection%20Enum :default "NewEnumerator0") (bEntering :type Boolean) (Key :type Key%20Structure :default "None") (bLoopingRepeat :type Boolean))
  ;[1 1 1] Globally call navigation input with valid check
  (bind _returnvalue (NiceSettingsMenu|GetNSMPCComponent))
  (Utilities|IsValid _returnvalue
    (:Is%20Valid
      (Default|NiceNaviagtionInput _returnvalue Direction bEntering Key bLoopingRepeat))))

(fn NiceNavigationAction
  (params (Action :type E_NiceNavigationAction%20Enum :default "NewEnumerator0") (bUseActiveWidget :type Boolean) (Widget :type WB%20Master%20Nav%20Widget%20Object%20Reference) (bEntering :type Boolean) (Key :type Key%20Structure :default "None"))
  ;[1 1 1] Globally call navigation action with valid check
  (bind _returnvalue (NiceSettingsMenu|GetNSMPCComponent))
  (Utilities|IsValid _returnvalue
    (:Is%20Valid
      (Default|NiceNavigationAction _returnvalue Action bUseActiveWidget Widget bEntering Key))))

(fn NiceNaviagtionNSMApplySetting
  (params (Key :type Key%20Structure :default "None") (bSwitchToKeyboardOrGamepadInput :type Boolean) (bShowConfirmAlertFirst :type Boolean))
  ;[1 1 1] Globally call navigation apply with valid check
  (bind _returnvalue (NiceSettingsMenu|GetNSMPCComponent))
  (Utilities|IsValid _returnvalue
    (:Is%20Valid
      (Default|NiceNavigationApplySettings _returnvalue Key bSwitchToKeyboardOrGamepadInput bShowConfirmAlertFirst))))

(fn NiceNavigationNSMRestoreDefaults
  (params (Key :type Key%20Structure :default "None") (bSwitchToKeyboardOrGamepadInput :type Boolean) (bShowConfirmAlertFirst :type Boolean))
  ;[1 1 1] Globally call navigation restore defaults with valid check
  (bind _returnvalue (NiceSettingsMenu|GetNSMPCComponent))
  (Utilities|IsValid _returnvalue
    (:Is%20Valid
      (Default|NiceNavigationRestoreDefaults _returnvalue Key bSwitchToKeyboardOrGamepadInput bShowConfirmAlertFirst))))

(fn NiceNaviagtionNSMResetSettings
  (params (Key :type Key%20Structure :default "None") (bSwitchToKeyboardOrGamepadInput :type Boolean) (bShowConfirmAlertFirst :type Boolean))
  ;[1 1 1] Globally call navigation reset settings with valid check
  (bind _returnvalue (NiceSettingsMenu|GetNSMPCComponent))
  (Utilities|IsValid _returnvalue
    (:Is%20Valid
      (Default|NiceNavigationResetSettings _returnvalue Key bSwitchToKeyboardOrGamepadInput bShowConfirmAlertFirst))))

(fn NiceNavigationShowStaticSettingInfo
  (params (bShow :type Boolean) (Key :type Key%20Structure :default "None"))
  ;[1 1 1] Globally call show static setting info with valid check
  (bind _returnvalue (NiceSettingsMenu|GetNSMPCComponent))
  (Utilities|IsValid _returnvalue
    (:Is%20Valid
      (Default|NiceNavigationShowStaticSettingInfo _returnvalue bShow Key))))

(fn NiceNavigationNSMSwitchSettingsSection
  (params (bForward :type Boolean) (Key :type Key%20Structure :default "None") (bSwitchToKeyboardOrGamepadInput :type Boolean))
  ;[1 1 1] Globally call go to next or previous settings section
  (bind _returnvalue (NiceSettingsMenu|GetNSMPCComponent))
  (Utilities|IsValid _returnvalue
    (:Is%20Valid
      (Default|NiceNavigationSwitchSettingsSection _returnvalue bForward Key bSwitchToKeyboardOrGamepadInput))))

(fn PlaySettingInteractionSound
  (params (ID :type Integer))
  ;[1 1 1] Small cooldown to prevent that interaction sound gets played multiple times at the same time
  (bind _returnvalue (NiceSettingsMenu|GetNSMPCComponent))
  (if (Variables|/Game/NiceSettingsMenu/Blueprints/AC_PC_NiceSettingsComponent.AC_PC_NiceSettingsComponent_C|GetbCanPlayInteractionSound _returnvalue)
    ;;[0.3687 0.4489 1] new in v1.1
    (bind _pausemenuref (Variables|/Game/NiceSettingsMenu/Blueprints/AC_PC_NiceSettingsComponent.AC_PC_NiceSettingsComponent_C|GetPauseMenuRef _returnvalue)
      (:then
        (Default|PauseMenuCooldownPlayInteractionSound _pausemenuref))
      (:else
        (Default|CooldownPlayInteractionSound _returnvalue)))
    (switch int ID ; You may want to have different\ninteraction sound effects
      (:0
        ;[1 1 1] Play interaction sound effect
        (Audio|PlaySound2D 0 "/Game/NiceSettingsMenu/Other/Sounds/SW_Click_01.SW_Click_01" 1.0 1.0 0.0 0 0)))))

(fn FindTextArrayElementIndex
  (params (Text :type Text) (TextArray :type Array%20of%20Texts))
  (for (_array_element _array_index) TextArray
    (if (Utilities|Enum|Equal(Enum) _array_element Text)
      (return _array_index)))
  (return -1))

(fn NSMSetWindowModeandScreenResolution
  (params (Resolution :type Text%20%28by%20ref%29) (WindowModeCode :type String) (bClampByMaxSupported :type Boolean))
  (bind _returnvalue (Utilities|String|ToString(Text) Resolution))
  (bind _returnvalue_2 (Utilities|String|ParseIntoArray _returnvalue "x"))
  (bind _output (Utilities|Array|Get(acopy) _returnvalue_2 1))
  (bind _output_2 (Utilities|Array|Get(acopy) _returnvalue_2))
  (bind _returnvalue_3 (Math|Conversions|ToInteger(Byte) _output))
  (bind _returnvalue_4 (Math|Conversions|ToInteger(Byte) _output_2))
  ;[1 1 1] Genrate resolution commmand and clamp resolution by max supported desktop screen resolution
  (bind _returnvalue_5 (Settings|GetGameUserSettings))
  ;[1 1 1] Execute command
  (bind _returnvalue_6 (NiceSettingsMenu|GetNSMPCComponent))
  (if (Utilities|Enum|NotEqual(Enum) (Variables|/Game/NiceSettingsMenu/Blueprints/AC_PC_NiceSettingsComponent.AC_PC_NiceSettingsComponent_C|GetLastWindowModeAndResCommand _returnvalue_6) (Utilities|String|Append "r.SetRes " (Utilities|String|Append (Utilities|String|ToString(Integer) (Math|Integer|SelectInt (Math|Integer|Clamp(Integer) _returnvalue_4 0 (.X (Utilities|Struct|BreakIntPoint (Class|GameUserSettings|GetDesktopResolution _returnvalue_5)))) _returnvalue_4 bClampByMaxSupported)) "x" (Utilities|String|ToString(Integer) (Math|Integer|SelectInt (Math|Integer|Clamp(Integer) _returnvalue_3 0 (.Y (Utilities|Struct|BreakIntPoint (Class|GameUserSettings|GetDesktopResolution _returnvalue_5)))) _returnvalue_3 bClampByMaxSupported))) WindowModeCode))
    (bind _output_get (Variables|/Game/NiceSettingsMenu/Blueprints/AC_PC_NiceSettingsComponent.AC_PC_NiceSettingsComponent_C|SetLastWindowModeAndResCommand _returnvalue_6 (Utilities|String|Append "r.SetRes " (Utilities|String|Append (Utilities|String|ToString(Integer) (Math|Integer|SelectInt (Math|Integer|Clamp(Integer) _returnvalue_4 0 (.X (Utilities|Struct|BreakIntPoint (Class|GameUserSettings|GetDesktopResolution _returnvalue_5)))) _returnvalue_4 bClampByMaxSupported)) "x" (Utilities|String|ToString(Integer) (Math|Integer|SelectInt (Math|Integer|Clamp(Integer) _returnvalue_3 0 (.Y (Utilities|Struct|BreakIntPoint (Class|GameUserSettings|GetDesktopResolution _returnvalue_5)))) _returnvalue_3 bClampByMaxSupported))) WindowModeCode)))
    (Development|ExecuteConsoleCommand 0 _output_get (Game|GetPlayerController 0))
    (Default|ExecuteCommandAfterTime _returnvalue_6 1.0 _output_get)
    ;[1 1 1] Debug
    (if (Variables|/Game/NiceSettingsMenu/Blueprints/AC_PC_NiceSettingsComponent.AC_PC_NiceSettingsComponent_C|GetbDebugAppliedSettings _returnvalue_6)
      (Development|PrintString 0 (Utilities|String|Append "Execute: " _output_get) true true "(R=1.000000,G=0.979922,B=0.947917,A=1.000000)"))))