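; Player controller for Decim8 that maps raw keyboard and gamepad keys to pause menu and settings menu controls.
; Escape and gamepad buttons reach the pause menu through ACPCNiceSettingsComponent, which also receives left-stick axes for navigation.
; Other keys call NiceNavigation helpers for directional movement, activation, setting info, section switching and confirm-first apply, reset and restore defaults.
; Gamepad Right Shoulder is bound to both reset settings and next section.
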(event EventBeginPlay)

(event Input|GamepadEvents|GamepadLeftX
  (params (AxisValue :type Float%20%28single-precision%29))
  ;[1 1 1] Keyboard & gamepad inputs for
  ; settings menu and nice navigation
  (Default|GamepadNiceNavX (Variables|Default|GetAC_PC_NiceSettingsComponent) AxisValue))

(event Input|GamepadEvents|GamepadLeftY
  (params (AxisValue :type Float%20%28single-precision%29))
  ;[1 1 1] Keyboard & gamepad inputs for
  ; settings menu and nice navigation
  (Default|GamepadNiceNavY (Variables|Default|GetAC_PC_NiceSettingsComponent) AxisValue))

(event Input|KeyboardEvents|R
  (params (Key :type Key%20Structure :default "None"))
  ;[1 1 1] Keyboard & gamepad inputs for
  ; settings menu and nice navigation
  (:Pressed
    (CallFunction|NiceNaviagtionNSMResetSettings Key true true)))

(event Input|KeyboardEvents|I
  (params (Key :type Key%20Structure :default "None"))
  ;[1 1 1] Keyboard & gamepad inputs for
  ; settings menu and nice navigation
  (:Pressed
    (CallFunction|NiceNavigationShowStaticSettingInfo true Key))
  (:Released
    (CallFunction|NiceNavigationShowStaticSettingInfo false Key)))

(event Input|GamepadEvents|GamepadFaceButtonBottom
  (params (Key :type Key%20Structure :default "None"))
  ;[1 1 1] Keyboard & gamepad inputs for
  ; settings menu and nice navigation
  (:Pressed
    (CallFunction|NiceNavigationAction "NewEnumerator0" true 0 true Key))
  (:Released
    (CallFunction|NiceNavigationAction "NewEnumerator0" true 0 false Key)))

(event Input|KeyboardEvents|Up
  (params (Key :type Key%20Structure :default "None"))
  ;[1 1 1] Keyboard & gamepad inputs for
  ; settings menu and nice navigation
  (:Pressed
    (CallFunction|NiceNaviagtionInput "NewEnumerator0" true Key true))
  (:Released
    (CallFunction|NiceNaviagtionInput "NewEnumerator0" false Key true)))

(event Input|KeyboardEvents|Right
  (params (Key :type Key%20Structure :default "None"))
  ;[1 1 1] Keyboard & gamepad inputs for
  ; settings menu and nice navigation
  (:Pressed
    (CallFunction|NiceNaviagtionInput "NewEnumerator3" true Key true))
  (:Released
    (CallFunction|NiceNaviagtionInput "NewEnumerator3" false Key true)))

(event Input|KeyboardEvents|Down
  (params (Key :type Key%20Structure :default "None"))
  ;[1 1 1] Keyboard & gamepad inputs for
  ; settings menu and nice navigation
  (:Pressed
    (CallFunction|NiceNaviagtionInput "NewEnumerator1" true Key true))
  (:Released
    (CallFunction|NiceNaviagtionInput "NewEnumerator1" false Key true)))

(event Input|KeyboardEvents|Left
  (params (Key :type Key%20Structure :default "None"))
  ;[1 1 1] Keyboard & gamepad inputs for
  ; settings menu and nice navigation
  (:Pressed
    (CallFunction|NiceNaviagtionInput "NewEnumerator2" true Key true))
  (:Released
    (CallFunction|NiceNaviagtionInput "NewEnumerator2" false Key true)))

(event Input|GamepadEvents|GamepadRightShoulder
  (params (Key :type Key%20Structure :default "None"))
  ;[1 1 1] Keyboard & gamepad inputs for
  ; settings menu and nice navigation
  (:Pressed
    (CallFunction|NiceNaviagtionNSMResetSettings Key true true)))

(event Input|GamepadEvents|GamepadDPadUp
  (params (Key :type Key%20Structure :default "None"))
  ;[1 1 1] Keyboard & gamepad inputs for
  ; settings menu and nice navigation
  (:Pressed
    (CallFunction|NiceNaviagtionInput "NewEnumerator0" true Key true))
  (:Released
    (CallFunction|NiceNaviagtionInput "NewEnumerator0" false Key true)))

(event Input|GamepadEvents|GamepadFaceButtonLeft
  (params (Key :type Key%20Structure :default "None"))
  ;[1 1 1] Keyboard & gamepad inputs for
  ; settings menu and nice navigation
  (:Pressed
    (CallFunction|NiceNaviagtionNSMApplySetting Key true true)))

(event Input|KeyboardEvents|A
  (params (Key :type Key%20Structure :default "None"))
  ;[1 1 1] Keyboard & gamepad inputs for
  ; settings menu and nice navigation
  (:Pressed
    (CallFunction|NiceNaviagtionNSMApplySetting Key true true)))

(event Input|KeyboardEvents|Enter
  (params (Key :type Key%20Structure :default "None"))
  ;[1 1 1] Keyboard & gamepad inputs for
  ; settings menu and nice navigation
  (:Pressed
    (CallFunction|NiceNavigationAction "NewEnumerator0" true 0 true Key))
  (:Released
    (CallFunction|NiceNavigationAction "NewEnumerator0" true 0 false Key)))

(event Input|GamepadEvents|GamepadRightTrigger
  (params (Key :type Key%20Structure :default "None"))
  ;[1 1 1] Keyboard & gamepad inputs for
  ; settings menu and nice navigation
  (:Pressed
    (CallFunction|NiceNavigationShowStaticSettingInfo true Key))
  (:Released
    (CallFunction|NiceNavigationShowStaticSettingInfo false Key)))

(event Input|GamepadEvents|GamepadSpecialRight
  (params (Key :type Key%20Structure :default "None"))
  ;[1 1 1] Open & Close Pause Menu
  (:Pressed
    (Default|OpenandClosePauseMenu (Default|GetPauseMenuRef (Variables|Default|GetAC_PC_NiceSettingsComponent)) "NewEnumerator1")))

(event Input|KeyboardEvents|Escape
  (params (Key :type Key%20Structure :default "None"))
  ;[1 1 1] Open & Close Pause Menu
  (:Pressed
    (Default|OpenandClosePauseMenu (Default|GetPauseMenuRef (Variables|Default|GetAC_PC_NiceSettingsComponent)) "NewEnumerator0")))

(event Input|GamepadEvents|GamepadLeftShoulder
  (params (Key :type Key%20Structure :default "None"))
  ;[1 1 1] Keyboard & gamepad inputs for
  ; settings menu and nice navigation
  (:Pressed
    (CallFunction|NiceNavigationNSMSwitchSettingsSection false Key true)))

(event Input|KeyboardEvents|Tab
  (params (Key :type Key%20Structure :default "None"))
  ;[1 1 1] Keyboard & gamepad inputs for
  ; settings menu and nice navigation
  (:Pressed
    (CallFunction|NiceNavigationNSMSwitchSettingsSection true Key false)))

(event Input|KeyboardEvents|1
  (params (Key :type Key%20Structure :default "None"))
  ;[1 1 1] Keyboard & gamepad inputs for
  ; settings menu and nice navigation
  (:Pressed
    (CallFunction|NiceNavigationNSMSwitchSettingsSection false "None" true)))

(event Input|KeyboardEvents|2
  (params (Key :type Key%20Structure :default "None"))
  ;[1 1 1] Keyboard & gamepad inputs for
  ; settings menu and nice navigation
  (:Pressed
    (CallFunction|NiceNavigationNSMSwitchSettingsSection true "None" true)))

(event Input|KeyboardEvents|D
  (params (Key :type Key%20Structure :default "None"))
  ;[1 1 1] Keyboard & gamepad inputs for
  ; settings menu and nice navigation
  (:Pressed
    (CallFunction|NiceNavigationNSMRestoreDefaults Key true true)))

(event Input|GamepadEvents|GamepadFaceButtonTop
  (params (Key :type Key%20Structure :default "None"))
  ;[1 1 1] Keyboard & gamepad inputs for
  ; settings menu and nice navigation
  (:Pressed
    (CallFunction|NiceNavigationNSMRestoreDefaults Key true true)))

(event Input|GamepadEvents|GamepadRightShoulder
  (params (Key :type Key%20Structure :default "None"))
  ;[1 1 1] Keyboard & gamepad inputs for
  ; settings menu and nice navigation
  (:Pressed
    (CallFunction|NiceNavigationNSMSwitchSettingsSection true Key true)))

(event Input|GamepadEvents|GamepadFaceButtonRight
  (params (Key :type Key%20Structure :default "None"))
  ;[1 1 1] Open & Close Pause Menu
  (:Pressed
    (Default|OpenandClosePauseMenu (Default|GetPauseMenuRef (Variables|Default|GetAC_PC_NiceSettingsComponent)) "NewEnumerator3")))

(event Input|GamepadEvents|GamepadDPadRight
  (params (Key :type Key%20Structure :default "None"))
  ;[1 1 1] Keyboard & gamepad inputs for
  ; settings menu and nice navigation
  (:Pressed
    (CallFunction|NiceNaviagtionInput "NewEnumerator3" true Key true))
  (:Released
    (CallFunction|NiceNaviagtionInput "NewEnumerator3" false Key true)))

(event Input|GamepadEvents|GamepadDPadDown
  (params (Key :type Key%20Structure :default "None"))
  ;[1 1 1] Keyboard & gamepad inputs for
  ; settings menu and nice navigation
  (:Pressed
    (CallFunction|NiceNaviagtionInput "NewEnumerator1" true Key true))
  (:Released
    (CallFunction|NiceNaviagtionInput "NewEnumerator1" false Key true)))

(event Input|GamepadEvents|GamepadDPadLeft
  (params (Key :type Key%20Structure :default "None"))
  ;[1 1 1] Keyboard & gamepad inputs for
  ; settings menu and nice navigation
  (:Pressed
    (CallFunction|NiceNaviagtionInput "NewEnumerator2" true Key true))
  (:Released
    (CallFunction|NiceNaviagtionInput "NewEnumerator2" false Key true)))

(fn ConstructionScript)